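; BP_ReflectionCapturer is a VLM sampler that measures brightness by rendering itself with a scene capture.
; The construction script limits the SceneCaptureComponent2D's show-only list to the actor itself.
; VLMCapture triggers a capture on demand, reads one render target pixel and returns its brightest channel with a fixed scale.
; A DebugValue event prints that result.
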(event Custom|Debug%20Value
  (bind _cpd_float_value (CallFunction|VLMCapture))
  (Development|PrintString (Utilities|String|ToString(Float) _cpd_float_value)))

(fn ConstructionScript
  (Variables|/Script/Engine.SceneCaptureComponent|SetShowOnlyActors (Variables|Default|GetSceneCaptureComponent2D) (Utilities|Array|MakeArray self)))

(fn VLMCapture
  (Rendering|SceneCapture|CaptureScene (Variables|Default|GetSceneCaptureComponent2D) :!class /Script/Engine.SceneCaptureComponent2D)
  (bind _returnvalue (Class|KismetRenderingLibrary|ReadRenderTargetPixel (Variables|/Script/Engine.SceneCaptureComponent2D|GetTextureTarget (Variables|Default|GetSceneCaptureComponent2D)) 1 1))
  (return (* (Class|KismetMathLibrary|LinearColorGetMax (Math|Conversions|ToLinearColor(Color) _returnvalue)) 1.5)))
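; Generated-mesh actor that builds light ray geometry aligned to a tagged sun actor's spot or directional light.
; A rotated, scaled rectangle is extruded along the light direction, then its vertices reshape a fresh UV-mapped box.
; The box loses its end caps and optional side pairs before receiving its material.
; BakeMesh saves it as a per-level static mesh asset and spawns a tagged, shadowless, distance-culled static actor.
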(event Custom|ResetMesh
  (bind _dynamicmesh (Variables|Default|GetDynamicMesh))
  (bind _rotation (Variables|Default|GetRotation))
  (bind _scale (Variables|Default|GetScale))
  (Rendering|SetVisibility (Variables|Default|GetDynamicMesh) true false)
  (bind _returnvalue (DynamicMeshComponent|GetDynamicMesh (Variables|DynamicMeshActor|GetDynamicMeshComponent)))
  (bind _returnvalue_2 (DynamicMesh|Reset _returnvalue))
  (Variables|Default|SetTarget%20Mesh _returnvalue_2)
  ;[1 1 1] Create Original Mesh with custom Rotate and Scale
  (bind _returnvalue_3 (Class|GeometryScriptLibraryMeshPrimitiveFunctions|AppendRectangleXY (Variables|Default|GetTarget%20Mesh) (Utilities|Struct|MakeGeometryScriptPrimitiveOptions "SingleGroup" true "Uniform") (Math|Transform|MakeTransform "0, 0, 0" "180.000000, 0, 0" "1.000000,1.000000,1.000000") (.x _scale) (.y _scale) 0 0 0))
  (bind _returnvalue_4 (GeometryScript|Transforms|TransformMesh _returnvalue_3 (Math|Transform|MakeTransform "0, 0, 0" (Math|Rotator|MakeRotator (.x _rotation) (.y _rotation) (.z _rotation)) "1.000000,1.000000,1.000000") true 0))
  ;[1 1 1] Lock Rotation and Scale on Mesh
  (Transformation|SetActorRotation "0, 0, 0")
  (Transformation|SetActorScale3D "1.000000,1.000000,1.000000")
  ;[1 1 1] Alt 1 -Get Sun Actor and Extrude Along Direction
  (bind _outactors (Actor|GetAllActorswithTag (Utilities|String|StringToName (Variables|Default|GetSun%20Tag))))
  (for (_array_element _array_index) _outactors
    (if (== (Utilities|GetClass _array_element) "/Script/Engine.SpotLight")
      (Variables|Default|SetOptions%20Extrude%20Direction (Math|Rotator|GetRotationXVector (Transformation|GetActorRotation (Utilities|Array|Get(acopy) _outactors _array_index))) :!label _label)
      (bind _returnvalue_5 (Class|GeometryScriptLibraryMeshModelingFunctions|ApplyMeshExtrudeCompatibility5p0 _returnvalue_4 (Utilities|Struct|MakeGeometryScriptMeshExtrudeOptions (.z _scale) (Variables|Default|GetOptions%20Extrude%20Direction) 1.0 true) 0 :!label _label_2))
      (bind _positionlist (GeometryScript|MeshQueries|GetAllVertexPositions _returnvalue_5))
      (bind _vectorarray (Class|GeometryScriptLibraryListUtilityFunctions|ConvertVectorListtoArray _positionlist))
      ;[1 1 1] Hide Original Mesh
      (Rendering|SetVisibility (Variables|DynamicMeshActor|GetDynamicMeshComponent) false false)
      (bind _returnvalue_6 (DynamicMeshComponent|GetDynamicMesh (Variables|Default|GetDynamicMesh)))
      (bind _returnvalue_7 (DynamicMesh|Reset _returnvalue_6))
      (bind _returnvalue_8 (Class|GeometryScriptLibraryMeshPrimitiveFunctions|AppendBox _returnvalue_7 (Utilities|Struct|MakeGeometryScriptPrimitiveOptions "PerFace" false "ScaleToFill") (Math|Transform|MakeTransform "0, 0, 0" "0, 0, 0" "1.000000,1.000000,1.000000") 1e+02 1e+02 1e+02 0 0 0 "Base" 0))
      (bind _returnvalue_9 (|SetVerticesPos _returnvalue_8 _vectorarray _vectorarray _vectorarray _vectorarray _vectorarray _vectorarray _vectorarray))
      ;[1 1 1] Delete Top and Bottom
      (for _index (range 1 2)
        (bind _returnvalue_10 (Class|GeometryScriptLibraryMeshPolygroupFunctions|DeleteTrianglesinPolygroup :TargetMesh _returnvalue_9 :PolygroupID _index :Debug 0)))
      ;[1 1 1] Optionally Delete Side Rays
      (if (Variables|Default|GetDelete%20X%20Sides)
        (for _index_2 (range 3 4)
          (Class|GeometryScriptLibraryMeshPolygroupFunctions|DeleteTrianglesinPolygroup :TargetMesh _returnvalue_10 :PolygroupID _index_2 :Debug 0)))
      (if (Variables|Default|GetDelete%20Y%20Sides)
        (for _index_3 (range 5 6)
          (Class|GeometryScriptLibraryMeshPolygroupFunctions|DeleteTrianglesinPolygroup :TargetMesh _returnvalue_10 :PolygroupID _index_3 :Debug 0)))
      (Class|GeometryScriptLibraryMeshNormalsFunctions|SetPerFaceNormals _returnvalue_10 0)
      (DynamicMeshComponent|GetDynamicMesh _dynamicmesh)
      ;[1 1 1] Set Material
      (if (Variables|Default|GetUse%20Debug%20Material)
        (Rendering|Material|SetMaterial _dynamicmesh 0 0)
        (else
          (Rendering|Material|SetMaterial _dynamicmesh 0 (Variables|Default|GetMaterial))))
      (elif (== (Utilities|GetClass _array_element) "/Script/Engine.DirectionalLight")
        (goto _label)
        (else
          ;[1 0 0] Alt 2 - Get Sun Actor Child Component and Extrude Along Direction
          (bind _returnvalue_11 (Class|EditorFilterLibrary|ByClass (Components|GetChildrenComponents (Variables|/Script/Engine.Actor|GetRootComponent _array_element) true) "/Script/Engine.SpotLightComponent" "Include"))
          (Variables|Default|SetOptions%20Extrude%20Direction (Math|Rotator|GetRotationXVector (Transformation|GetWorldRotation (Utilities|Array|Get(acopy) _returnvalue_11))))
          (if (Math|Conversions|ToBoolean(Integer) (Utilities|Array|Length _returnvalue_11))
            (goto _label_2)
            (else
              (bind _returnvalue_12 (Class|EditorFilterLibrary|ByClass (Components|GetChildrenComponents (Variables|/Script/Engine.Actor|GetRootComponent _array_element) true) "/Script/Engine.DirectionalLightComponent" "Include"))
              (Variables|Default|SetOptions%20Extrude%20Direction (Math|Rotator|GetRotationXVector (Transformation|GetWorldRotation (Utilities|Array|Get(acopy) _returnvalue_12))))
              (if (Math|Conversions|ToBoolean(Integer) (Utilities|Array|Length _returnvalue_12))
                (goto _label_2)))))))))

(event Events|EventOnRebuildGeneratedMesh
  (params (TargetMesh :type Dynamic%20Mesh%20Object%20Reference))
  (bind _dynamicmesh (Variables|Default|GetDynamicMesh))
  (bind _rotation (Variables|Default|GetRotation))
  (bind _scale (Variables|Default|GetScale))
  (Variables|Default|SetTarget%20Mesh TargetMesh)
  ;[1 1 1] Create Original Mesh with custom Rotate and Scale
  (bind _returnvalue (Class|GeometryScriptLibraryMeshPrimitiveFunctions|AppendRectangleXY (Variables|Default|GetTarget%20Mesh) (Utilities|Struct|MakeGeometryScriptPrimitiveOptions "SingleGroup" true "Uniform") (Math|Transform|MakeTransform "0, 0, 0" "180.000000, 0, 0" "1.000000,1.000000,1.000000") (.x _scale) (.y _scale) 0 0 0))
  (bind _returnvalue_2 (GeometryScript|Transforms|TransformMesh _returnvalue (Math|Transform|MakeTransform "0, 0, 0" (Math|Rotator|MakeRotator (.x _rotation) (.y _rotation) (.z _rotation)) "1.000000,1.000000,1.000000") true 0))
  ;[1 1 1] Lock Rotation and Scale on Mesh
  (Transformation|SetActorRotation "0, 0, 0")
  (Transformation|SetActorScale3D "1.000000,1.000000,1.000000")
  ;[1 1 1] Alt 1 -Get Sun Actor and Extrude Along Direction
  (bind _outactors (Actor|GetAllActorswithTag (Utilities|String|StringToName (Variables|Default|GetSun%20Tag))))
  (for (_array_element _array_index) _outactors
    (if (== (Utilities|GetClass _array_element) "/Script/Engine.SpotLight")
      (Variables|Default|SetOptions%20Extrude%20Direction (Math|Rotator|GetRotationXVector (Transformation|GetActorRotation (Utilities|Array|Get(acopy) _outactors _array_index))) :!label _label)
      (bind _returnvalue_3 (Class|GeometryScriptLibraryMeshModelingFunctions|ApplyMeshExtrudeCompatibility5p0 _returnvalue_2 (Utilities|Struct|MakeGeometryScriptMeshExtrudeOptions (.z _scale) (Variables|Default|GetOptions%20Extrude%20Direction) 1.0 true) 0 :!label _label_2))
      (bind _positionlist (GeometryScript|MeshQueries|GetAllVertexPositions _returnvalue_3))
      (bind _vectorarray (Class|GeometryScriptLibraryListUtilityFunctions|ConvertVectorListtoArray _positionlist))
      ;[1 1 1] Hide Original Mesh
      (Rendering|SetVisibility (Variables|DynamicMeshActor|GetDynamicMeshComponent) false false)
      (bind _returnvalue_4 (DynamicMeshComponent|GetDynamicMesh (Variables|Default|GetDynamicMesh)))
      (bind _returnvalue_5 (DynamicMesh|Reset _returnvalue_4))
      (bind _returnvalue_6 (Class|GeometryScriptLibraryMeshPrimitiveFunctions|AppendBox _returnvalue_5 (Utilities|Struct|MakeGeometryScriptPrimitiveOptions "PerFace" false "ScaleToFill") (Math|Transform|MakeTransform "0, 0, 0" "0, 0, 0" "1.000000,1.000000,1.000000") 1e+02 1e+02 1e+02 0 0 0 "Base" 0))
      (bind _returnvalue_7 (|SetVerticesPos _returnvalue_6 _vectorarray _vectorarray _vectorarray _vectorarray _vectorarray _vectorarray _vectorarray))
      ;[1 1 1] Delete Top and Bottom
      (for _index (range 1 2)
        (bind _returnvalue_8 (Class|GeometryScriptLibraryMeshPolygroupFunctions|DeleteTrianglesinPolygroup :TargetMesh _returnvalue_7 :PolygroupID _index :Debug 0)))
      ;[1 1 1] Optionally Delete Side Rays
      (if (Variables|Default|GetDelete%20X%20Sides)
        (for _index_2 (range 3 4)
          (Class|GeometryScriptLibraryMeshPolygroupFunctions|DeleteTrianglesinPolygroup :TargetMesh _returnvalue_8 :PolygroupID _index_2 :Debug 0)))
      (if (Variables|Default|GetDelete%20Y%20Sides)
        (for _index_3 (range 5 6)
          (Class|GeometryScriptLibraryMeshPolygroupFunctions|DeleteTrianglesinPolygroup :TargetMesh _returnvalue_8 :PolygroupID _index_3 :Debug 0)))
      (Class|GeometryScriptLibraryMeshNormalsFunctions|SetPerFaceNormals _returnvalue_8 0)
      (DynamicMeshComponent|GetDynamicMesh _dynamicmesh)
      ;[1 1 1] Set Material
      (if (Variables|Default|GetUse%20Debug%20Material)
        (Rendering|Material|SetMaterial _dynamicmesh 0 0)
        (else
          (Rendering|Material|SetMaterial _dynamicmesh 0 (Variables|Default|GetMaterial))))
      (elif (== (Utilities|GetClass _array_element) "/Script/Engine.DirectionalLight")
        (goto _label)
        (else
          ;[1 0 0] Alt 2 - Get Sun Actor Child Component and Extrude Along Direction
          (bind _returnvalue_9 (Class|EditorFilterLibrary|ByClass (Components|GetChildrenComponents (Variables|/Script/Engine.Actor|GetRootComponent _array_element) true) "/Script/Engine.SpotLightComponent" "Include"))
          (Variables|Default|SetOptions%20Extrude%20Direction (Math|Rotator|GetRotationXVector (Transformation|GetWorldRotation (Utilities|Array|Get(acopy) _returnvalue_9))))
          (if (Math|Conversions|ToBoolean(Integer) (Utilities|Array|Length _returnvalue_9))
            (goto _label_2)
            (else
              (bind _returnvalue_10 (Class|EditorFilterLibrary|ByClass (Components|GetChildrenComponents (Variables|/Script/Engine.Actor|GetRootComponent _array_element) true) "/Script/Engine.DirectionalLightComponent" "Include"))
              (Variables|Default|SetOptions%20Extrude%20Direction (Math|Rotator|GetRotationXVector (Transformation|GetWorldRotation (Utilities|Array|Get(acopy) _returnvalue_10))))
              (if (Math|Conversions|ToBoolean(Integer) (Utilities|Array|Length _returnvalue_10))
                (goto _label_2)))))))))

(fn ConstructionScript)

(fn BakeMesh
  (bind _returnvalue (Game|GetCurrentLevelName true))
  (bind _returnvalue_2 (DynamicMeshComponent|GetDynamicMesh (Variables|Default|GetDynamicMesh)))
  (bind _returnvalue_3 (GeometryScript|AssetManagement|CreateNewStaticMeshAssetfromMesh _returnvalue_2 (Utilities|String|Append (Utilities|String|MakeLiteralString "/Game/Environment/GeneratedMeshes/") (Utilities|String|Append (Utilities|String|Append _returnvalue "_") (Utilities|GetObjectName self))) (Utilities|Struct|MakeGeometryScriptCreateNewStaticMeshAssetOptions false false false "(bEnabled=False,bPreserveArea=False,PositionPrecision=-2147483648,NormalPrecision=-1,TargetMinimumResidencyInKB=0,KeepPercentTriangles=1.000000,TrimRelativeError=0.000000,FallbackPercentTriangles=1.000000,FallbackRelativeError=1.000000,DisplacementUVChannel=0,DisplacementMaps=)" 0.0 false "CTF_UseDefault") 0)
    (:Success
      (Class|EditorAssetLibrary|CheckoutLoadedAsset _returnvalue_3)
      (EditorScripting|Asset|SaveLoadedAsset _returnvalue_3 :!class /Script/EditorScriptingUtilities.EditorAssetLibrary)
      (bind _returnvalue_4 (Class|EditorLevelLibrary|SpawnActorfromObject _returnvalue_3 (Transformation|GetActorLocation self) "0, 0, 0" false))
      (bind _asstatic_mesh_actor (Utilities|Casting|CastToStaticMeshActor _returnvalue_4))
      (Variables|/Script/Engine.Actor|SetTags _asstatic_mesh_actor (Utilities|Array|MakeArray "lightray_static"))
      (Utilities|FlowControl|Sequence
        (:then_0
          ;[1 1 1] Set Material
          (if (Variables|Default|GetUse%20Debug%20Material)
            (Rendering|Material|SetMaterial (Variables|/Script/Engine.StaticMeshActor|GetStaticMeshComponent _asstatic_mesh_actor) 0 "/Game/MaterialLibrary/M_Default_CustomUV_2Sided.M_Default_CustomUV_2Sided")
            (else
              (Rendering|Material|SetMaterial (Variables|/Script/Engine.StaticMeshActor|GetStaticMeshComponent _asstatic_mesh_actor) 0 (Variables|Default|GetMaterial)))))
        (:then_1
          ;[1 1 1] Set Visibility
          (Rendering|SetVisibility (Variables|Default|GetDynamicMesh) false false)
          (Rendering|SetVisibility (Variables|/Script/Engine.StaticMeshActor|GetStaticMeshComponent _asstatic_mesh_actor) true false))
        (:then_2
          ;[1 1 1] Set Mobility and Draw Distance
          (Transformation|SetMobility (Variables|/Script/Engine.StaticMeshActor|GetStaticMeshComponent _asstatic_mesh_actor) "Static")
          (Class|PrimitiveComponent|SetCullDistance (Variables|/Script/Engine.StaticMeshActor|GetStaticMeshComponent _asstatic_mesh_actor) (Variables|Default|GetMax%20Draw%20Distance)))
        (:then_3
          ;[1 1 1] Turn off Shadows
          (Rendering|SetCastShadow (Variables|/Script/Engine.StaticMeshActor|GetStaticMeshComponent _asstatic_mesh_actor) false))))))